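; Draggable actor that the player picks up with a left click and moves with the mouse along a fixed X plane.
; OnClicked, rebound every Tick, sets IsMoving, and the completed or canceled IA_LeftClick input clears it.
; While moving, a camera-to-cursor Visibility trace sets the root's Y and Z, with X locked to Plan.
; Interpolated, pathing and force-based movement alternatives remain disconnected in Move.
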(event Custom|OnClicked_Event
  (params (TouchedActor :type Actor%20Object%20Reference) (ButtonPressed :type Key%20Structure :default "None"))
  ;[0.15 0.15 0.15 0.5] Grab
  (CallFunction|Grab))

(event Custom|IsClicked
  ;[0.15 0.15 0.15 0.5] Grab
  (EventDispatchers|BindEventtoOnClicked (delegate Custom|OnClicked_Event)))

(event Input|EnhancedActionEvents|EnhancedInputActionIA_LeftClick
  (params (ActionValue :type Boolean) (ElapsedSeconds :type Float%20%28double-precision%29) (TriggeredSeconds :type Float%20%28double-precision%29) (InputAction :type Input%20Action%20Object%20Reference :default "/Game/GaetanProjectCPP/Actions/Inputs/IA_LeftClick.IA_LeftClick"))
  ;[0.15 0.15 0.15 0.5] Grab
  (:Canceled
    (CallFunction|Ungrab :!label _label))
  (:Completed
    (goto _label)))

(event EventBeginPlay
  (Input|EnableInput (Game|GetPlayerController 0)))

(event EventTick
  (params (DeltaSeconds :type Float%20%28single-precision%29))
  ;[0.15 0.15 0.15 0.5] Movement
  (CallFunction|IsClicked)
  (CallFunction|Move))

(fn ConstructionScript)

(fn Move
  (bind _returnvalue (Game|GetPlayerController 0))
  (bind (_locationx _locationy) (Game|Player|GetMousePosition _returnvalue))
  (bind _playercameramanager (Variables|/Script/Engine.PlayerController|GetPlayerCameraManager _returnvalue))
  (bind _returnvalue_2 (Camera|GetCameraLocation _playercameramanager))
  (if (Variables|Default|GetIsMoving)
    (bind _outhit (Collision|LineTraceByChannel _returnvalue_2 (+ _returnvalue_2 (* 1e+04 (.WorldDirection (Class|GameplayStatics|DeprojectScreentoWorld _returnvalue (Math|Vector2D|MakeVector2D _locationx _locationy))))) "TraceTypeQuery1" false 0 "None"))
    (Transformation|SetWorldLocation (Variables|Default|GetDefaultSceneRoot) (Math|Vector|MakeVector (Variables|Default|GetPlan) (.Y (Math|Vector|BreakVector (.ImpactPoint (Collision|BreakHitResult _outhit)))) (.Z (Math|Vector|BreakVector (.ImpactPoint (Collision|BreakHitResult _outhit))))) false false)))

(fn Grab
  (Variables|Default|SetIsMoving true))

(fn Ungrab
  (Variables|Default|SetIsMoving false))