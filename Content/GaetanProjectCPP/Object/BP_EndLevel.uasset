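; BP_EndLevel is an end-of-level trigger that sends the player to the next level when BP_Player overlaps its Box.
; EndLevel opens LevelToLoad, banks the timer, then sets the GameManager's CurrentLevel to NextLevelID.
; SetTotalTimer adds the level time to TotalTimer, stores it in the LevelTimer array at the finished level's index, and resets CurrentLevelTimer.
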(event OnComponentBeginOverlap(Box)
  (params (OverlappedComponent :type Primitive%20Component%20Object%20Reference) (OtherActor :type Actor%20Object%20Reference) (OtherComp :type Primitive%20Component%20Object%20Reference) (OtherBodyIndex :type Integer) (bFromSweep :type Boolean) (SweepResult :type Hit%20Result%20Structure%20%28by%20ref%29))
  (Utilities|Casting|CastToBP_Player OtherActor)
  (CallFunction|EndLevel))

(event EventBeginPlay)

(event Collision|EventActorBeginOverlap
  (params (OtherActor :type Actor%20Object%20Reference)))

(event EventTick
  (params (DeltaSeconds :type Float%20%28single-precision%29)))

(fn ConstructionScript)

(fn EndLevel
  (Game|OpenLevel(byObjectReference) (Variables|Default|GetLevelToLoad))
  (CallFunction|SetTotalTimer)
  (Variables|/Script/GaetanProjectCPP.GameManager|Set_currentLevel (Subsystems|GetGameManager) (Variables|Default|GetNextLevelID)))

(fn SetTotalTimer
  (bind _returnvalue (Subsystems|GetGameManager))
  (Variables|/Script/GaetanProjectCPP.GameManager|Set_totalTimer _returnvalue (+ (Variables|/Script/GaetanProjectCPP.GameManager|Get_currentLevelTimer _returnvalue) (Variables|/Script/GaetanProjectCPP.GameManager|Get_totalTimer _returnvalue)))
  (Utilities|Array|SetArrayElem (Variables|/Script/GaetanProjectCPP.GameManager|Get_levelTimer _returnvalue) (Variables|/Script/GaetanProjectCPP.GameManager|Get_currentLevel _returnvalue) (Variables|/Script/GaetanProjectCPP.GameManager|Get_currentLevelTimer _returnvalue))
  (Variables|/Script/GaetanProjectCPP.GameManager|Set_currentLevelTimer _returnvalue 0.0))