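; BP_Bille is a grabbable colored ball (pink, green or blue) that fuses with another ball to spawn a platform object.
; Color sets the material and a power-of-two ColorID, so each pair's sum is unique.
; Overlap tracks the fusion partner; ungrabbing over one looks that sum up in DT_BilleFusion and spawns the matching class.
; Both balls are destroyed even without a matching row; otherwise ungrab falls back to the parent.
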(event OnComponentBeginOverlap(Collision)
  (params (OverlappedComponent :type Primitive%20Component%20Object%20Reference) (OtherActor :type Actor%20Object%20Reference) (OtherComp :type Primitive%20Component%20Object%20Reference) (OtherBodyIndex :type Integer) (bFromSweep :type Boolean) (SweepResult :type Hit%20Result%20Structure%20%28by%20ref%29))
  ;[0.15 0.15 0.15 0.5] Collision
  (bind _asbp_bille (Utilities|Casting|CastToBP_Bille OtherActor))
  (Variables|Default|SetBilleToFusion _asbp_bille))

(event OnComponentEndOverlap(Collision)
  (params (OverlappedComponent :type Primitive%20Component%20Object%20Reference) (OtherActor :type Actor%20Object%20Reference) (OtherComp :type Primitive%20Component%20Object%20Reference) (OtherBodyIndex :type Integer))
  ;[0.15 0.15 0.15 0.5] Collision
  (bind _asbp_bille (Utilities|Casting|CastToBP_Bille OtherActor))
  (if (== _asbp_bille (Variables|Default|GetBilleToFusion))
    (Variables|Default|SetBilleToFusion 0)))

(event EventBeginPlay
  ;[0.15 0.15 0.15 0.5] Set Up
  (|CallParentFunction)
  (CallFunction|InitialiseColor (Variables|Default|GetColor)))

(fn ConstructionScript)

(fn InitialiseColor
  (params (Color :type EBilleColor%20Enum :default "NewEnumerator0"))
  (bind _sphere (Variables|Default|GetSphere))
  (Variables|Default|SetBilleToFusion 0)
  (bind _output_get (Variables|Default|SetColor Color))
  (switch Utilities|FlowControl|Switch|SwitchonEBilleColor _output_get
    (:NewEnumerator0
      (Rendering|Material|SetMaterial _sphere 0 (Variables|Materials|GetPinkMat))
      (Variables|Default|SetColorID 1))
    (:NewEnumerator1
      (Rendering|Material|SetMaterial _sphere 0 (Variables|Materials|GetGreenMat))
      (Variables|Default|SetColorID 2))
    (:NewEnumerator2
      (Rendering|Material|SetMaterial _sphere 0 (Variables|Materials|GetBlueMat))
      (Variables|Default|SetColorID 4))))

(fn Fusion
  (bind _billetofusion (Variables|Default|GetBilleToFusion))
  (bind _colorid (Variables|Default|GetColorID))
  (bind _colorid_2 (Variables|BP_Bille_C|GetColorID _billetofusion))
  (bind _returnvalue (+ _colorid _colorid_2))
  (bind _returnvalue_2 (Utilities|GetDataTableRow "/Game/GaetanProjectCPP/Object/Billes/DT_BilleFusion.DT_BilleFusion" (Utilities|String|StringToName (Utilities|String|ToString(Integer) _returnvalue)))
    (:then
      (bind _returnvalue_3 (Game|SpawnActorfromClass (.plateforme_object _returnvalue_2) (Transformation|GetActorTransform) "Undefined" "MultiplyWithRoot" 0 0))
      (Default|Initialise _returnvalue_3 _returnvalue))
    (:RowNotFound
      _))
  (Actor|DestroyActor (Variables|Default|GetBilleToFusion))
  (Actor|DestroyActor))

(fn Ungrab
  (Utilities|IsValid (Variables|Default|GetBilleToFusion)
    (:Is%20Valid
      (CallFunction|Fusion))
    (:Is%20Not%20Valid
      (|CallParentFunction))))

(fn Initialise
  (params (SpawnLocationY :type Float%20%28double-precision%29) (SpawnLocationZ :type Float%20%28double-precision%29) (Color :type EBilleColor%20Enum :default "NewEnumerator0"))
  (Transformation|SetActorLocation (Math|Vector|MakeVector (Variables|Default|GetPlan) SpawnLocationY SpawnLocationZ) false false)
  (CallFunction|InitialiseColor Color))