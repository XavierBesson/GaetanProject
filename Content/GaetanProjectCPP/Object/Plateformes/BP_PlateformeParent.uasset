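; BP_PlateformeParent is a base Blueprint for grabbable platforms that can split back into two BP_Bille balls.
; Grab makes it transparent and lets pawns pass through; Ungrab restores opaque, blocking behavior.
; Initialise stores its ID and snaps its X position to the Plan coordinate.
; Right-clicking while IsMoving triggers Defusion, which looks up that ID in DT_BilleFusion, spawns both source colors side by side, and destroys the platform.
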(event Input|EnhancedActionEvents|EnhancedInputActionIA_RightClick
  (params (ActionValue :type Boolean) (ElapsedSeconds :type Float%20%28double-precision%29) (TriggeredSeconds :type Float%20%28double-precision%29) (InputAction :type Input%20Action%20Object%20Reference :default "/Game/GaetanProjectCPP/Actions/Inputs/IA_RightClick.IA_RightClick"))
  (:Started
    (if (Variables|Default|GetIsMoving)
      (CallFunction|Defusion))))

(event EventBeginPlay
  (|CallParentFunction)
  (Rendering|Material|SetMaterial (Variables|Default|GetStaticMesh) 0 (Variables|Default|GetOpaqueMaterial)))

(event EventTick
  (params (DeltaSeconds :type Float%20%28single-precision%29))
  (|CallParentFunction DeltaSeconds))

(fn ConstructionScript)

(fn Defusion
  (bind _returnvalue (Transformation|GetActorLocation))
  (bind _returnvalue_2 (Utilities|GetDataTableRow "/Game/GaetanProjectCPP/Object/Billes/DT_BilleFusion.DT_BilleFusion" (Utilities|String|StringToName (Utilities|String|ToString(Integer) (Variables|Default|GetID))))
    (:then
      (bind _returnvalue_3 (Game|SpawnActorfromClass "/Game/GaetanProjectCPP/Object/Billes/BP_Bille.BP_Bille_C" (Math|Transform|MakeTransform "0, 0, 0" "0, 0, 0" "1.000000,1.000000,1.000000") "Undefined" "MultiplyWithRoot" 0 0))
      (Default|Initialise _returnvalue_3 (- (.y _returnvalue) 3e+01) (.z _returnvalue) (.firstbille _returnvalue_2))
      (bind _returnvalue_4 (Game|SpawnActorfromClass "/Game/GaetanProjectCPP/Object/Billes/BP_Bille.BP_Bille_C" (Math|Transform|MakeTransform "0, 0, 0" "0, 0, 0" "1.000000,1.000000,1.000000") "Undefined" "MultiplyWithRoot" 0 0))
      (Default|Initialise _returnvalue_4 (+ (.y _returnvalue) 3e+01) (.z _returnvalue) (.secondbille _returnvalue_2))
      (Actor|DestroyActor))))

(fn Grab
  (|CallParentFunction)
  (Collision|SetCollisionResponsetoChannel (Variables|Default|GetCollision) "ECC_Pawn" "ECR_Ignore")
  (Rendering|Material|SetMaterial (Variables|Default|GetStaticMesh) 0 (Variables|Default|GetTransparentMaterial)))

(fn Ungrab
  (|CallParentFunction)
  (Collision|SetCollisionResponsetoChannel (Variables|Default|GetStaticMesh) "ECC_Pawn" "ECR_Block")
  (Rendering|Material|SetMaterial (Variables|Default|GetStaticMesh) 0 (Variables|Default|GetOpaqueMaterial)))

(fn Initialise
  (params (ID :type Integer))
  (bind _returnvalue (Transformation|GetActorLocation))
  (Variables|Default|SetID ID)
  (Transformation|SetActorLocation (Math|Vector|MakeVector (Variables|Default|GetPlan) (.y _returnvalue) (.z _returnvalue)) false false))