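; BP_VerticalPlateforme is a moving platform actor that travels along a spline, reversing at each end.
; On BeginPlay it attaches the Platform component to the Spline.
; Every Tick, MoveOnSpline advances a distance by speed and direction, then places the platform at that spline point in local space without sweep.
; The distance is clamped at both ends, and the step ignores delta time, so speed depends on frame rate.
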(event EventBeginPlay
  (|CallParentFunction)
  (Transformation|AttachComponentToComponent (Variables|Default|GetPlatform) (Variables|Default|GetSpline) "None" "KeepRelative" "KeepRelative" "KeepRelative" true))

(event Collision|EventActorBeginOverlap
  (params (OtherActor :type Actor%20Object%20Reference))
  (|CallParentFunction OtherActor) ; This node is disabled and will not be called.\nDrag off pins to build functionality.
)

(event EventTick
  (params (DeltaSeconds :type Float%20%28single-precision%29))
  (|CallParentFunction DeltaSeconds)
  (CallFunction|MoveonSpline))

(fn ConstructionScript
  (|CallParentFunction))

(fn MoveonSpline
  (bind _spline (Variables|Default|GetSpline))
  (bind _returnvalue (Spline|GetSplineLength _spline))
  (bind _output_get (Variables|Spline|SetDistance (+ (Variables|Spline|GetDistance) (* (Variables|Spline|GetSplineSpeed) (Variables|Spline|GetDirection)))))
  (Transformation|SetRelativeLocation (Variables|Default|GetPlatform) (Spline|GetLocationatDistanceAlongSpline _spline _output_get "Local") false false)
  (if (>= (Variables|Spline|GetDistance) _returnvalue)
    (Variables|Spline|SetDistance _returnvalue)
    (Math|Float|NegateFloat (Variables|Spline|GetDirection) :!label _label)
    (elif (<= (Variables|Spline|GetDistance) 0.0)
      (Variables|Spline|SetDistance 0.0)
      (goto _label))))