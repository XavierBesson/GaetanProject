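; BP_PivotPlateforme is a platform actor that rocks back and forth around its roll axis.
; Every Tick, Rotation adds Direction times Speed to the platform's relative roll, without scaling by delta time.
; ChangeDirection then checks the roll against MaxAngle times Direction and flips Direction once that limit is passed, producing a continuous pivot.
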(event EventBeginPlay
  (|CallParentFunction) ; This node is disabled and will not be called.\nDrag off pins to build functionality.
)

(event Collision|EventActorBeginOverlap
  (params (OtherActor :type Actor%20Object%20Reference))
  (|CallParentFunction OtherActor) ; This node is disabled and will not be called.\nDrag off pins to build functionality.
)

(event EventTick
  (params (DeltaSeconds :type Float%20%28single-precision%29))
  (|CallParentFunction DeltaSeconds)
  (CallFunction|Rotation))

(fn ConstructionScript
  (|CallParentFunction))

(fn Rotation
  (bind _platform (Variables|Default|GetPlatform))
  (bind _relativerotation (Variables|/Script/Engine.SceneComponent|GetRelativeRotation _platform))
  (Transformation|SetRelativeRotation _platform (Math|Rotator|MakeRotator (+ (.roll _relativerotation) (* (Variables|Rotation|GetDirection) (Variables|Rotation|GetSpeed))) (.pitch _relativerotation) (.yaw _relativerotation)) false false)
  (CallFunction|ChangeDirection))

(fn ChangeDirection
  (bind _platform (Variables|Default|GetPlatform))
  (bind _relativerotation (Variables|/Script/Engine.SceneComponent|GetRelativeRotation _platform))
  (if (>= (Variables|Rotation|GetDirection) 0.0)
    (if (> (.roll _relativerotation) (* (Variables|Rotation|GetMaxAngle) (Variables|Rotation|GetDirection)))
      (Math|Float|NegateFloat (Variables|Rotation|GetDirection) :!label _label))
    (elif (< (.roll _relativerotation) (* (Variables|Rotation|GetMaxAngle) (Variables|Rotation|GetDirection)))
      (goto _label))))